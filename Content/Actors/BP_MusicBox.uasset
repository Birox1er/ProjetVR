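; BP_MusicBox is a music box actor linked to the crank system with ID 1.
; On BeginPlay it starts MusicTime at 15, finds tagged CrankSystem actors and binds to that system's state updates.
; Updates with exactly one grabbed crank are forwarded to OnCrankStateUpdated, and Tick prints MusicTime for debugging.
; The click handler that sets MusicTime is never bound, and InitCrankLink is empty.
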(event Custom|CustomEvent
  (params (IsRunning :type Boolean) (CranksGrabbed :type Integer))
  (if (== CranksGrabbed 1)
    (Class|AMusicBox|OnCrankStateUpdated IsRunning CranksGrabbed)))

(event Custom|OnClicked_Event
  (params (TouchedActor :type Actor%20Object%20Reference) (ButtonPressed :type Key%20Structure :default "None"))
  (Development|PrintString "Hello")
  (Class|AMusicBox|SetMusicTime 1e+01))

(event EventBeginPlay
  (Variables|Default|SetMusicTime 15.0)
  (bind _outactors (Actor|GetAllActorswithTag "CrankSystem"))
  (for _array_element _outactors
    (bind _asbp_crank_system (Utilities|Casting|CastToBP_CrankSystem _array_element))
    (if (== (Variables|/Game/LevelPrototyping/Blueprints/BP_CrankSystem.BP_CrankSystem_C|GetSystemID _asbp_crank_system) 1)
      (EventDispatchers|BindEventtoOnCrankStateUpdate _asbp_crank_system (delegate Custom|CustomEvent)))))

(event EventTick
  (params (DeltaSeconds :type Float%20%28single-precision%29))
  (Development|PrintString (Utilities|String|Append "Music time :" (Utilities|String|ToString(Float) (Variables|Default|GetMusicTime))) true true "(R=0.000000,G=0.983743,B=1.000000,A=1.000000)" 0.1 "MusicTime"))

(fn ConstructionScript)

(fn InitCrankLink)